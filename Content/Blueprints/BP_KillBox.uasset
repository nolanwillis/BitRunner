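; BP_KillBox is a kill volume that marks any BP_Bit entering its collider as dead and drops it downward.
; On overlap it stores the bit, sets IsDead and computes an end point FallDistance below its location.
; A Timeline then lerps the bit to that point without sweeping.
; One stored reference and Timeline serve all overlaps, so a new bit takes over any fall in progress.
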(event `self.Collider.OnComponentBeginOverlap`
  (params (OverlappedComponent :type "PrimitiveComponent Object Reference") (OtherActor :type "Actor Object Reference") (OtherComp :type "PrimitiveComponent Object Reference") (OtherBodyIndex :type Integer) (bFromSweep :type Boolean) (SweepResult :type "HitResult Structure (by ref)"))
  (bind _asbp_bit (cast `/Game/Blueprints/BP_Bit` OtherActor))
  (bind _output_get (set `self.BP_Bit` _asbp_bit))
  (set `Bit.bIsDead` true _output_get)
  (bind _output_get_2 (set `self.FallStartLoc` (`self.K2_GetActorLocation` _asbp_bit)))
  (set `self.FallEndLoc` (`KismetMathLibrary.MakeVector` (.x _output_get_2) (.y _output_get_2) (- (.z _output_get_2) (`self.FallDistance`))))
  (bind (_direction _value) (`Timeline|Timeline` :!via `PlayFromStart`)
    (:`Update`
      (`self.K2_SetActorLocation` (`self.BP_Bit`) (`KismetMathLibrary.VLerp` (`self.FallStartLoc`) (`self.FallEndLoc`) _value) false false))))

(fn `UserConstructionScript`)