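; BP_Bit is the BitRunner player Blueprint, and its only logic is taking damage.
; On AnyDamage it skips the hit while Immune is set, otherwise it subtracts the damage from CurrentHealth, clamped at zero.
; Each outcome shows an on-screen debug print of either the immunity or the new health, and nothing here handles death at zero health.
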(event `self.ReceiveAnyDamage`
  (params (Damage :type "Float (single-precision)") (DamageType :type "DamageType Object Reference") (InstigatedBy :type "Controller Object Reference") (DamageCauser :type "Actor Object Reference"))
  (bind _returnvalue (- (`self.CurrentHealth`) Damage))
  (if (`self.bImmune`)
    (`KismetSystemLibrary.PrintString` "IMMUNE" true false (struct :`G` 0.578545 :`B` 1.0 :`A` 1.0))
    (elif (>= _returnvalue 0.0)
      (bind _output_get (set `self.CurrentHealth` _returnvalue))
      (`KismetSystemLibrary.PrintString` (`KismetStringLibrary.Conv_DoubleToString` _output_get) true false (struct :`R` 1.0 :`B` 0.008466 :`A` 1.0))
      (else
        (bind _output_get_2 (set `self.CurrentHealth` 0.0))
        (`KismetSystemLibrary.PrintString` (`KismetStringLibrary.Conv_DoubleToString` _output_get_2) true false (struct :`R` 1.0 :`B` 0.016558 :`A` 1.0))))))

(fn `UserConstructionScript`)