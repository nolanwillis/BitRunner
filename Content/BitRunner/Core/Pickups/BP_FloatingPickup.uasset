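; BP_FloatingPickup is a pickup actor that bobs up and down and spins in place, with no collection logic in its graphs.
; Tick adds the change in a sine of the actor's lifetime, scaled by FloatAmount, to its current height.
; It also advances yaw by RotationSpeed scaled by delta time, applying location and rotation in one call.
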(event `self.ReceiveBeginPlay`)

(event `self.ReceiveTick`
  (params (DeltaSeconds :type "Float (single-precision)"))
  (bind _returnvalue (`self.GetGameTimeSinceCreation`))
  (set `self.CurrentRotation` (`self.K2_GetActorRotation`))
  (set `self.CurrentLocation` (`self.K2_GetActorLocation`))
  (set `self.DeltaHeight` (- (`KismetMathLibrary.Sin` (+ _returnvalue DeltaSeconds)) (`KismetMathLibrary.Sin` _returnvalue)))
  (set `self.DeltaRotation` (* (`self.RotationSpeed`) DeltaSeconds))
  (`self.K2_SetActorLocationAndRotation` (`KismetMathLibrary.MakeVector` (.x (`self.CurrentLocation`)) (.y (`self.CurrentLocation`)) (+ (.z (`self.CurrentLocation`)) (* (`self.DeltaHeight`) (`self.FloatAmount`)))) (`KismetMathLibrary.MakeRotator` (.roll (`self.CurrentRotation`)) (.pitch (`self.CurrentRotation`)) (+ (.yaw (`self.CurrentRotation`)) (`self.DeltaRotation`)))))

(fn `UserConstructionScript`)