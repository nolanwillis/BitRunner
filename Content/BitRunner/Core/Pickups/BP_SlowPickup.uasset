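; BP_SlowPickup is a BitRunner pickup that temporarily slows the BP_Bit that overlaps it.
; On collider overlap it stores the Bit's MovementSpeedX, halves it and hides its three static meshes.
; A short one-shot timer then restores the stored speed and destroys the pickup, which stays alive but invisible until then.
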(event `self.ReceiveTick`
  (params (DeltaSeconds :type "Float (single-precision)"))
  (`parent.ReceiveTick` DeltaSeconds))

(event `self.Collider.OnComponentBeginOverlap`
  (params (OverlappedComponent :type "PrimitiveComponent Object Reference") (OtherActor :type "Actor Object Reference") (OtherComp :type "PrimitiveComponent Object Reference") (OtherBodyIndex :type Integer) (bFromSweep :type Boolean) (SweepResult :type "HitResult Structure (by ref)"))
  (bind _movementspeedx (`Bit.MovementSpeedX` (`self.As BP Bit`)))
  (bind _asbp_bit (cast `/Game/BitRunner/Core/Player/BP_Bit` OtherActor))
  (set `self.As BP Bit` _asbp_bit)
  (set `self.OriginalSpeed` _movementspeedx)
  (set `Bit.MovementSpeedX` (/ _movementspeedx 2.0) (`self.As BP Bit`))
  (`KismetSystemLibrary.K2_SetTimerDelegate` (delegate `ResetMovementSpeedX`) 2.0)
  (`SceneComponent.SetVisibility` (`self.StaticMesh`) false false)
  (`SceneComponent.SetVisibility` (`self.StaticMesh2`) false false)
  (`SceneComponent.SetVisibility` (`self.StaticMesh3`) false false))

(event `ResetMovementSpeedX`
  (set `Bit.MovementSpeedX` (`self.OriginalSpeed`) (`self.As BP Bit`))
  (`self.K2_DestroyActor`))

(fn `UserConstructionScript`
  (`parent.UserConstructionScript`))