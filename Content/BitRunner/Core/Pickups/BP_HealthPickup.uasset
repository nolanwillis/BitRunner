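; BP_HealthPickup is a pickup that restores health to the player's BP_Bit when touched.
; On collider overlap it casts the other actor to BP_Bit and adds HealthAmount to CurrentHealth, capped at MaxHealth.
; It then destroys itself and prints the new health value on screen in green.
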(event `self.ReceiveTick`
  (params (DeltaSeconds :type "Float (single-precision)"))
  (`parent.ReceiveTick` DeltaSeconds))

(event `self.Collider.OnComponentBeginOverlap`
  (params (OverlappedComponent :type "PrimitiveComponent Object Reference") (OtherActor :type "Actor Object Reference") (OtherComp :type "PrimitiveComponent Object Reference") (OtherBodyIndex :type Integer) (bFromSweep :type Boolean) (SweepResult :type "HitResult Structure (by ref)"))
  (bind _bp_bit (`self.BP_Bit`))
  (bind _bp_bit_2 (`self.BP_Bit`))
  (bind _maxhealth (`Bit.MaxHealth` _bp_bit_2))
  (bind _returnvalue (+ (`Bit.CurrentHealth` _bp_bit_2) (`self.HealthAmount`)))
  (bind _asbp_bit (cast `/Game/BitRunner/Core/Player/BP_Bit` OtherActor))
  (set `self.BP_Bit` _asbp_bit)
  (if (<= _returnvalue _maxhealth)
    (bind _output_get (set `Bit.CurrentHealth` _returnvalue _bp_bit))
    (else
      (set `Bit.CurrentHealth` _maxhealth _bp_bit)))
  (`self.K2_DestroyActor`)
  (`KismetSystemLibrary.PrintString` (`KismetStringLibrary.Conv_DoubleToString` _output_get) true false (struct :`G` 1.0 :`B` 0.00301 :`A` 1.0)))

(fn `UserConstructionScript`
  (`parent.UserConstructionScript`))