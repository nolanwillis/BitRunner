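; Floor section of an endless track that spawns its successor at its attach point, quickly while fewer than fifteen sections exist, slower otherwise.
; On BeginPlay it randomly places a health or slow pickup and scatters damage boxes or rarer kill boxes across child spawn points.
; When BP_Bit leaves the main collider it expires shortly after; re-entering clears that lifespan.
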(event `self.ReceiveBeginPlay`
  (`self.SpawnRandomPickup`)
  (`self.SpawnRandomObstacles`)
  (bind _outactors (`GameplayStatics.GetAllActorsOfClass` "BP_Floor1_C"))
  (if (>= (`KismetArrayLibrary.Array_Length` _outactors) 15)
    (`KismetSystemLibrary.K2_SetTimerDelegate` (delegate `SpawnNextSection`) 10.0)
    (else
      (`KismetSystemLibrary.K2_SetTimerDelegate` (delegate `SpawnNextSection`) 1.0))))

(event `SpawnNextSection`
  (bind _attachpoint (`self.AttachPoint`))
  (`|SpawnActorFromClass` "BP_Floor1_C" (`KismetMathLibrary.MakeTransform` (`SceneComponent.K2_GetComponentLocation` _attachpoint) (`SceneComponent.K2_GetComponentRotation` _attachpoint)) "Undefined" "OverrideRootScale" null null))

(event `self.MainCollider.OnComponentEndOverlap`
  (params (OverlappedComponent :type "PrimitiveComponent Object Reference") (OtherActor :type "Actor Object Reference") (OtherComp :type "PrimitiveComponent Object Reference") (OtherBodyIndex :type Integer))
  (cast `/Game/BitRunner/Core/Player/BP_Bit` OtherActor)
  (`self.SetLifeSpan` 0.9))

(event `self.MainCollider.OnComponentBeginOverlap`
  (params (OverlappedComponent :type "PrimitiveComponent Object Reference") (OtherActor :type "Actor Object Reference") (OtherComp :type "PrimitiveComponent Object Reference") (OtherBodyIndex :type Integer) (bFromSweep :type Boolean) (SweepResult :type "HitResult Structure (by ref)"))
  (cast `/Game/BitRunner/Core/Player/BP_Bit` OtherActor)
  (`self.SetLifeSpan` 0.0))

(fn `SpawnRandomObstacles`
  (locals (SpawnLocation :type "Vector Structure" :default (0.0 0.0 0.0)))
  (for _array_element (`SceneComponent.GetChildrenComponents` (`self.ObstacleSpawnPoints`) false)
    (if (== (`KismetMathLibrary.RandomIntegerInRange` 0 2) 0)
      (if (== (`KismetMathLibrary.RandomIntegerInRange` 0 5) 0)
        (bind _returnvalue (`SceneComponent.K2_GetComponentLocation` _array_element))
        (`|SpawnActorFromClass` "/Game/BitRunner/Core/Obstacles/BP_KillBox.BP_KillBox_C" (`KismetMathLibrary.MakeTransform` _returnvalue) "Undefined" "OverrideRootScale" null null)
        (else
          (`|SpawnActorFromClass` "/Game/BitRunner/Core/Obstacles/BP_DamageBox.BP_DamageBox_C" (`KismetMathLibrary.MakeTransform` _returnvalue) "Undefined" "OverrideRootScale" null null))))))

(fn `SpawnRandomPickup`
  (locals (RandomSpawnPoint :type "Vector Structure") (NewLocalVar :type "Vector Structure"))
  (bind _returnvalue (`KismetMathLibrary.RandomIntegerInRange` 0 1))
  (if (== (`KismetMathLibrary.RandomIntegerInRange` 0 4) 0)
    (set `local.RandomSpawnPoint` (`SceneComponent.K2_GetComponentLocation` (`KismetArrayLibrary.Array_Random` (`SceneComponent.GetChildrenComponents` (`self.PickupSpawnPoints`) false))))
    (if (== _returnvalue 0)
      (`|SpawnActorFromClass` "/Game/BitRunner/Core/Pickups/BP_HealthPickup.BP_HealthPickup_C" (`KismetMathLibrary.MakeTransform` (`local.RandomSpawnPoint`)) "Undefined" "OverrideRootScale" null null)
      (elif (== _returnvalue 1)
        (`|SpawnActorFromClass` "/Game/BitRunner/Core/Pickups/BP_SlowPickup.BP_SlowPickup_C" (`KismetMathLibrary.MakeTransform` (`local.RandomSpawnPoint`)) "Undefined" "OverrideRootScale" null null)))))

(fn `UserConstructionScript`)